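; BP_Rifle_SN is a rifle pickup that spins in place and can spawn projectiles.
; On overlap, ServerOverlap runs with authority, calling WeaponAttachment on a BP_PlayerCharacter_SN and destroying the pickup, unless the character's PickupWeapon equals a particular enum value.
; The starfire event spawns BP_Projectile_SN using MuzzleRotation and the StaticMesh's transform, as no socket is named.
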(event `self.ReceiveActorBeginOverlap`
  (params (OtherActor :type "Actor Object Reference"))
  (`self.ServerOverlap` OtherActor))

(event `self.ReceiveTick`
  (params (DeltaSeconds :type "Float (single-precision)"))
  ;[1 1 1] WeaponRotation
  (`self.K2_AddActorLocalRotation` (* (`self.WeaponRotateSpeed`) (`GameplayStatics.GetWorldDeltaSeconds`))))

(event `ServerOverlap`
  (params (Actor :type "Actor Object Reference"))
  (`/Engine/EditorBlueprintResources/ActorMacros.Switch Has Authority`
    (:`Authority`
      (`/Engine/EditorBlueprintResources/StandardMacros.IsValid` Actor
        (:`Is Valid`
          (bind _asbp_player_character_sn (cast `/Game/SN/Blueprints_SN/BP_PlayerCharacter_SN` Actor))
          (if (not (`|EnumEquality` (`/Game/SN/Blueprints_SN/BP_PlayerCharacter_SN.PickupWeapon` _asbp_player_character_sn) "NewEnumerator3"))
            (`/Game/SN/Blueprints_SN/BP_PlayerCharacter_SN.WeaponAttachment` _asbp_player_character_sn)
            (`self.K2_DestroyActor`)))))))

(event `starfire`
  (`|SpawnActorFromClass` "/Game/SN/Blueprints_SN/BP_Projectile_SN.BP_Projectile_SN_C" (`KismetMathLibrary.MakeTransform` (.location (`SceneComponent.GetSocketTransform` (`self.StaticMesh`) "None" "RTS_World")) (`self.MuzzleRotation`)) "AlwaysSpawn" "OverrideRootScale" null null))

(fn `UserConstructionScript`)