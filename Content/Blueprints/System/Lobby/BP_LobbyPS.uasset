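; BP_LobbyPS is the lobby player state, storing each player's UID and skin selection.
; It sets UI-only input for non-octopus lobby controllers on BeginPlay.
; Where the lobby game mode is absent, as on clients, it copies UID and skin into BP_GI and calls the controller's SetMeshAndMatServer.
; SetMeshAndMaterial applies the skin to the pawn, switches to game-only input, then attaches weapons after a short delay.
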(event `self.ReceiveBeginPlay`
  (bind _asbp_lobby_pc (cast `/Game/Blueprints/System/Lobby/BP_LobbyPC` (`self.GetOwner`)))
  (bind _isoctopus (`/Game/Blueprints/System/Lobby/BP_LobbyPC.IsOctopus_LobbyPC` _asbp_lobby_pc))
  (if (not _isoctopus)
    (`WidgetBlueprintLibrary.SetInputMode_UIOnlyEx` _asbp_lobby_pc null)))

(event `SetLocalInfoToClientGI`
  (cast `/Game/Blueprints/System/Lobby/BP_LobbyGM` (`GameplayStatics.GetGameMode`)
    (:`CastFailed`
      (bind _asbp_gi (cast `/Game/Blueprints/Public/BP_GI` (`GameplayStatics.GetGameInstance`)))
      (`/Engine/EditorBlueprintResources/StandardMacros.IsValid` _asbp_gi
        (:`Is Valid`
          (`/Game/Blueprints/Public/BP_GI.SetLocalUID` _asbp_gi (`self.UID`))
          (set `/Game/Blueprints/Public/BP_GI.LocalSkinState` (`self.LocalSkinState`) _asbp_gi)
          (bind _asbp_lobby_pc (cast `/Game/Blueprints/System/Lobby/BP_LobbyPC` (`self.GetOwner`)))
          (`/Engine/EditorBlueprintResources/StandardMacros.IsValid` _asbp_lobby_pc
            (:`Is Valid`
              (`/Game/Blueprints/System/Lobby/BP_LobbyPC.SetMeshAndMatServer` _asbp_lobby_pc))))))))

(event `SetMeshAndMaterial`
  (bind _asbp_player_character_sn (cast `/Game/SN/Blueprints_SN/BP_PlayerCharacter_SN` (`self.PawnPrivate`)))
  (`/Engine/EditorBlueprintResources/StandardMacros.IsValid` _asbp_player_character_sn
    (:`Is Valid`
      (bind _result (`/Game/Blueprints/Skin/BP_SkinData.GetSkinStruct` (`self.BP_SkinData`) (`self.LocalSkinState`)))
      (bind _mesh (`Character.Mesh` _asbp_player_character_sn))
      (bind (_skin _mesh_2 _mat) (break `/Game/Blueprints/Skin/SkinStruct` _result))
      (`SkinnedMeshComponent.SetSkinnedAssetAndUpdate` _mesh _mesh_2 true)
      (`PrimitiveComponent.SetMaterial` _mesh 0 _mat)
      (bind _asbp_lobby_pc (cast `/Game/Blueprints/System/Lobby/BP_LobbyPC` (`self.GetOwner`)))
      (`WidgetBlueprintLibrary.SetInputMode_GameOnly` _asbp_lobby_pc)
      (`KismetSystemLibrary.Delay` 0.2)
      (`/Game/SN/Blueprints_SN/BP_PlayerCharacter_SN.WeaponAttachment` _asbp_player_character_sn))))

(fn `SetLocalSkinState`
  (params (SkinState :type "/Game/Blueprints/Skin/ESkinState Enum" :default "NewEnumerator0"))
  (set `self.LocalSkinState` SkinState))

(fn `SetUID`
  (params (NewUID :type Integer))
  (set `self.UID` NewUID))

(fn `UserConstructionScript`)